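; BP_GrapplingPoint is a grapple target actor with a mesh, a collision sphere and a widget component marker.
; BeginPlay caches the widget's draw size and hands the mesh to BP_GrapplingWidget as its parent reference.
; Each Tick copies CharacterFocused to the widget and then clears it, so focus must be re-asserted externally every frame.
; Tick also collapses the sphere's radius to zero when the player pawn is out of range.
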(event EventBeginPlay
  (bind _grapplewidget (Variables|Default|GetGrappleWidget))
  (bind _returnvalue (Class|WidgetComponent|GetDrawSize _grapplewidget))
  (bind (_x _y) (Math|Vector2D|BreakVector2D _returnvalue))
  (Variables|Default|SetBaseDrawSizeY _y)
  (Variables|Default|SetBaseDrawSizeX _x)
  (bind _asbp_grappling_widget (Utilities|Casting|CastToBP_GrapplingWidget (UserInterface|GetUserWidgetObject (Variables|Default|GetGrappleWidget))))
  (Variables|/Game/Grappling/HUD/BP_GrapplingWidget.BP_GrapplingWidget_C|SetParentRef _asbp_grappling_widget (Variables|Default|GetGrappleMesh)))

(event Collision|EventActorBeginOverlap
  (params (OtherActor :type Actor%20Object%20Reference)))

(event EventTick
  (params (DeltaSeconds :type Float%20%28single-precision%29))
  (bind _asbp_grappling_widget (Utilities|Casting|CastToBP_GrapplingWidget (UserInterface|GetUserWidgetObject (Variables|Default|GetGrappleWidget))))
  (Variables|/Game/Grappling/HUD/BP_GrapplingWidget.BP_GrapplingWidget_C|SetFocused _asbp_grappling_widget (Variables|Default|GetbCharacterFocused))
  (Variables|Default|SetbCharacterFocused false)
  (if (> (Transformation|GetDistanceTo (Game|Player|GetPlayerPawn 0)) 1e+03)
    (Components|Sphere|SetSphereRadius (Variables|Default|GetCollisionSphere) 0.0 true)
    (else
      (Components|Sphere|SetSphereRadius (Variables|Default|GetCollisionSphere) 64.0 true))))

(fn ConstructionScript)